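; BP_InfantryW2 is an infantry enemy AI that senses, approaches and shoots the player, with extra Life added on spawn.
; PawnSensing detection sets SeeTarget and starts AIMoveTo toward the player pawn, while a delayed Tick keeps it facing the player.
; A looping timer calls Fire, spawning LaserIA projectiles from Arrow1 while alive and within range.
; An empty magazine triggers a timed reload, mirrored to the Blackboard's isReloading key.
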(event `self.ReceiveBeginPlay`
  (`|ExecutionSequence`
    (:`then_0`
      (`KismetSystemLibrary.K2_SetTimer` null "Fire" 0.5 true))
    (:`then_1`
      (set `self.Life` (+ (`self.Life`) 20.0)))))

(event `Reload`
  (if (not (or (`self.IsReloading`) (`self.Isdead_0`)))
    (`BlackboardComponent.SetValueAsBool` (`AIBlueprintHelperLibrary.GetBlackboard` (`self.GetController`)) "isReloading" true)
    (set `self.IsReloading` true)
    (`KismetSystemLibrary.Delay` 2.5)
    (set `self.AmmoInMag` (`self.MaxAmmoInMag`))
    (set `self.IsReloading` false)
    (`BlackboardComponent.SetValueAsBool` (`AIBlueprintHelperLibrary.GetBlackboard` (`self.GetController`)) "isReloading" false)))

(event `Fire`
  (if (and (>= (`self.Life`) 1.0) (`self.SeeTarget`))
    (if (== (`self.AmmoInMag`) 0)
      (`self.Reload`)
      (elif (< (`KismetMathLibrary.VSize` (- (`self.K2_GetActorLocation` (`GameplayStatics.GetPlayerPawn` 0)) (`self.K2_GetActorLocation`))) 1500.0)
        (`|SpawnActorFromClass` "/Game/PFE/Blueprint/BulletsOrWeapon/Bullets/LaserIA.LaserIA_C" (`SceneComponent.K2_GetComponentToWorld` (`self.Arrow1`)) "Undefined" "OverrideRootScale" null null)
        (set `self.AmmoInMag` (- (`self.AmmoInMag`) 1))))))

(event `self.PawnSensing.OnSeePawn`
  (params (Pawn :type "Pawn Object Reference"))
  (bind _asbp_world_interaction_pawn (cast `/Game/PFE/Blueprint/J1/BP_WorldInteractionPawn` Pawn))
  (bind _returnvalue (`self.K2_GetActorLocation` _asbp_world_interaction_pawn))
  (`self.K2_SetActorRotation` (`KismetMathLibrary.FindLookAtRotation` (`self.K2_GetActorLocation`) _returnvalue))
  (set `self.SeeTarget` true)
  (`|AIMoveTo` self _returnvalue _asbp_world_interaction_pawn 1000.0))

(event `self.ReceiveTick`
  (params (DeltaSeconds :type "Float (single-precision)"))
  (`KismetSystemLibrary.Delay` 0.2)
  (bind _asbp_world_interaction_pawn (cast `/Game/PFE/Blueprint/J1/BP_WorldInteractionPawn` (`GameplayStatics.GetPlayerPawn` 0)))
  (`self.K2_SetActorRotation` (`KismetMathLibrary.FindLookAtRotation` (`self.K2_GetActorLocation`) (`self.K2_GetActorLocation` _asbp_world_interaction_pawn))))

(fn `UserConstructionScript`
  (`parent.UserConstructionScript`))