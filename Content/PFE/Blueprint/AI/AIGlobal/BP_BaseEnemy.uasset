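; BP_BaseEnemy is an enemy character that loses Life to tagged player weapons and turrets, then dissolves on death.
; Capsule overlaps apply damage by tag, while Sphere overlaps deal heavier laser damage into the same death check.
; Surviving hits briefly highlight the mesh through custom depth stencil.
; Lethal hits trigger physics and an impulse, then timeline-driven material dissolve and destruction; "Black" overlaps skip straight to the dissolve.
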(event `self.CapsuleComponent.OnComponentBeginOverlap`
  (params (OverlappedComponent :type "PrimitiveComponent Object Reference") (OtherActor :type "Actor Object Reference") (OtherComp :type "PrimitiveComponent Object Reference") (OtherBodyIndex :type Integer) (bFromSweep :type Boolean) (SweepResult :type "HitResult Structure (by ref)"))
  (bind _mesh (`self.Mesh`))
  ;[1 1 1] Take Damage / Die
  (if (or (`self.ActorHasTag` OtherActor "Laser") (`ActorComponent.ComponentHasTag` OtherComp "Laser"))
    (set `self.Life` (- (`self.Life`) 30.0))
    (if (<= (`self.Life`) 0.0) :!label _label
      (`PrimitiveComponent.SetSimulatePhysics` (`self.Mesh`) true)
      (`PrimitiveComponent.SetSimulatePhysics` (`self.CapsuleComponent`) true)
      (`PrimitiveComponent.AddImpulse` (`self.CapsuleComponent`) (-600.0 0.0 0.0) "None" false)
      (`PrimitiveComponent.SetCollisionEnabled` (`self.CapsuleComponent`) "QueryAndPhysics")
      (`KismetSystemLibrary.Delay` 7.0)
      (bind _returnvalue (`PrimitiveComponent.CreateDynamicMaterialInstance` (`self.Mesh`) 0 null "None" :!label _label_2))
      (set `self.Isdead` true)
      (bind (_direction _newtrack_0) (`Timeline|Timeline_0`)
        (:`Update`
          (`MaterialInstanceDynamic.SetScalarParameterValue` _returnvalue "amount" _newtrack_0)
          (bind _returnvalue_2 (`PrimitiveComponent.CreateDynamicMaterialInstance` (`self.Mesh`) 1 null "None"))
          (bind (_direction_2 _newtrack_0_2) (`Timeline|Timeline_1`)
            (:`Update`
              (`MaterialInstanceDynamic.SetScalarParameterValue` _returnvalue_2 "amount" _newtrack_0_2)
              (`KismetSystemLibrary.Delay` 1.5)
              (`self.K2_DestroyActor`)))))
      (else
        (`PrimitiveComponent.SetRenderCustomDepth` _mesh true)
        (`PrimitiveComponent.SetCustomDepthStencilValue` (`self.Mesh`) 2)
        (`KismetSystemLibrary.Delay` 3.0)
        (`PrimitiveComponent.SetRenderCustomDepth` _mesh false)
        (`PrimitiveComponent.SetCustomDepthStencilValue` _mesh 2)))
    (elif (or (`self.ActorHasTag` OtherActor "LaserVR") (`self.ActorHasTag` OtherActor "LaserTurret"))
      (set `self.Life` (- (`self.Life`) 30.0))
      (goto _label)
      (elif (`self.ActorHasTag` OtherActor "Scan")
        _
        (elif (or (`self.ActorHasTag` OtherActor "Claw") (`ActorComponent.ComponentHasTag` OtherComp "Sword"))
          (set `self.Life` (- (`self.Life`) 100.0))
          (goto _label)
          (elif (`self.ActorHasTag` OtherActor "Black")
            (goto _label_2)))))))

(event `self.Sphere.OnComponentBeginOverlap`
  (params (OverlappedComponent :type "PrimitiveComponent Object Reference") (OtherActor :type "Actor Object Reference") (OtherComp :type "PrimitiveComponent Object Reference") (OtherBodyIndex :type Integer) (bFromSweep :type Boolean) (SweepResult :type "HitResult Structure (by ref)"))
  ;[1 1 1] Take Damage / Die
  (if (`self.ActorHasTag` OtherActor "Laser")
    (set `self.Life` (- (`self.Life`) 50.0))
    (goto _label)
    (elif (`self.ActorHasTag` OtherActor "LaserTurret")
      (set `self.Life` (- (`self.Life`) 100.0))
      (goto _label))))

(event `self.ReceiveBeginPlay`
  (bind _asgame_instance_pfe (cast `/Game/PFE/Blueprint/GameInstance/GameInstance_PFE` (`GameplayStatics.GetGameInstance`)))
  (set `self.GI` _asgame_instance_pfe))

(event `self.ReceiveTick`
  (params (DeltaSeconds :type "Float (single-precision)")))

(fn `UserConstructionScript`)