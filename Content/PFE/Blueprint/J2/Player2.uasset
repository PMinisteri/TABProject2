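; Player 2's flying character, with boost, looping-timer laser fire, pausing and an attachable turret mode.
; Interacting inside a "Slot" overlap locks movement, switches fire to turret lasers and changes the custom-depth stencil.
; Firing and turret mode spend Energy, with Shield draining once it empties; a Delay-throttled Tick regenerates Energy, Shield and Life while CalmDown is set.
; "LaserIA" hits reduce Shield, then Life, teleporting the player to a fixed point at zero.
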(event `self.ReceiveEndPlay`
  (params (EndPlayReason :type "EEndPlayReason Enum" :default "Destroyed"))
  ;[1 1 1] Event End Play
  (`QuitMatchCallbackProxy.QuitMatch` null))

(event `self.ReceiveBeginPlay`
  ;[1 1 1] Event begin play
  (bind _asbp_world_interaction_pawn (cast `/Game/PFE/Blueprint/J1/BP_WorldInteractionPawn` (`self.VRPlayer`)))
  (set `self.VRPlayer` _asbp_world_interaction_pawn)
  (bind _asgame_instance_pfe (cast `/Game/PFE/Blueprint/GameInstance/GameInstance_PFE` (`GameplayStatics.GetGameInstance`)))
  (set `self.GI` _asgame_instance_pfe)
  (bind _aslaser (cast `/Game/PFE/Blueprint/BulletsOrWeapon/Bullets/Laser` (`self.Laser`)))
  (set `self.Laser` _aslaser)
  (if (`self.IsLocallyControlled`)
    _))

(event `InteractBoolean`
  (set `self.Interact` true :!label _label))

(event `InputAction|P2Interact`
  (params (Key :type "Key Structure"))
  (:`Pressed`
    (goto _label))
  (:`Released`
    (set `self.Interact` false :!label _label_2)))

(event `InputAction|Boost`
  (params (Key :type "Key Structure"))
  ;[1 1 1] Boost
  (:`Pressed`
    (`self.Sprint`))
  (:`Released`
    (`self.NoSprint`)))

(event `Sprint`
  ;[1 1 1] Boost
  (set `CharacterMovementComponent.MaxFlySpeed` 1500.0 (`self.CharacterMovement`)))

(event `InteractBooleanFalse`
  (goto _label_2))

(event `Key|P`
  (params (Key :type "Key Structure"))
  ;[1 0.8266 0] Input Pause (Keep or not ?)
  (:`Pressed`
    (`/Engine/EditorBlueprintResources/StandardMacros.FlipFlop` :!label _label_3
      (:`A`
        (`self.PauseGame`)))))

(event `NoSprint`
  ;[1 1 1] Boost
  (set `CharacterMovementComponent.MaxFlySpeed` 600.0 (`self.CharacterMovement`)))

(event `InputAction|Pause`
  (params (Key :type "Key Structure"))
  ;[1 0.8266 0] Input Pause (Keep or not ?)
  (:`Pressed`
    (goto _label_3)))

(event `PauseGame`
  ;[1 0.8266 0] Input Pause (Keep or not ?)
  (`GameplayStatics.SetGamePaused` true)
  (bind _returnvalue (`|CreateWidget` "/Game/PFE/Blueprint/Widget/P2/PauseMenu.PauseMenu_C"))
  (`UserWidget.AddToViewport` _returnvalue 0)
  (`WidgetBlueprintLibrary.SetInputMode_UIOnlyEx` (`GameplayStatics.GetPlayerController` 0) null)
  (set `PlayerController.bShowMouseCursor` true (`GameplayStatics.GetPlayerController` 0)))

(event `self.ReceiveActorBeginOverlap`
  (params (OtherActor :type "Actor Object Reference"))
  ;[1 0.6223 0.5322] TurretCondition
  (if (`self.ActorHasTag` OtherActor "Slot")
    (if (and (or (>= (`self.Energy`) 1.0) (>= (`self.Shield`) 1.0)) (not (`self.DoShoot`)))
      (set `self.TurretOK?` true))
    (elif (`self.ActorHasTag` OtherActor "LaserIA")
      (`self.Die` null)
      (set `self.TakeDamage` true)
      (`KismetSystemLibrary.Delay` 1.5)
      (set `self.TakeDamage` false))))

(event `InputAxis|MoveForward`
  (params (AxisValue :type "Float (single-precision)"))
  ;[1 1 1] Movement
  (if (not (`self.Attach`))
    (`self.AddMovementInput` (`KismetMathLibrary.GetForwardVector` (`KismetMathLibrary.MakeRotator` 0.0 (.pitch (`self.GetControlRotation`)) (.yaw (`self.GetControlRotation`)))) AxisValue)))

(event `Die`
  (params (Target :type "Actor Object Reference") (Tag :type Name))
  (bind _life (`self.Life`))
  ;[1 1 1] Die/Regen Event
  (if (>= (`self.Shield`) 0.0)
    (set `self.Shield` (- (`self.Shield`) 2.0))
    (set `self.CalmDown` false :!label _label_4)
    (`KismetSystemLibrary.Delay` 1.0)
    (if (not (`self.TakeDamage`))
      (set `self.CalmDown` true))
    (else
      (set `self.Life` (- _life 1.0))
      (if (<= _life 0.0)
        (`self.K2_SetActorLocation` (-4854.0 -1618.0 2000.0) false true)
        (goto _label_4)))))

(event `self.ReceiveActorEndOverlap`
  (params (OtherActor :type "Actor Object Reference"))
  ;[1 0.6223 0.5322] TurretCondition
  (if (`self.ActorHasTag` OtherActor "Slot")
    (set `self.TurretOK?` false)))

(event `InputAxis|MoveRight`
  (params (AxisValue :type "Float (single-precision)"))
  ;[1 1 1] Movement
  (if (not (`self.Attach`))
    (`self.AddMovementInput` (`KismetMathLibrary.GetRightVector` (`KismetMathLibrary.MakeRotator` 0.0 (.pitch (`self.GetControlRotation`)) (.yaw (`self.GetControlRotation`)))) AxisValue)))

(event `InputAction|Fire`
  (params (Key :type "Key Structure"))
  ;[0.4078 1 0.4995] ShootGestion
  (:`Pressed`
    (if (`self.Attach`)
      (`self.PullTurret`)
      (set `self.CalmDown` false)
      (else
        (`self.PullTrigger`)
        (set `self.CalmDown` false)
        (set `self.DoShoot` true))))
  (:`Released`
    (if (`self.Attach`)
      (`self.ReleaseTurret`)
      (set `self.DoShoot` false)
      (set `self.CalmDown` false)
      (else
        (`self.ReleaseTrigger`)
        (set `self.DoShoot` false)
        (`KismetSystemLibrary.Delay` 1.0)
        (if (not (`self.DoShoot`))
          (set `self.CalmDown` true))))))

(event `Regen`
  ;[0 0.6384 1] LifeGestion
  (`KismetSystemLibrary.Delay` 1.2)
  (set `self.Life` (+ (`self.Life`) 3.0)))

(event `InputAxis|GoUp`
  (params (AxisValue :type "Float (single-precision)"))
  ;[1 1 1] Go up / Go down
  (if (not (`self.Attach`))
    (`self.AddMovementInput` (`KismetMathLibrary.GetUpVector` (`KismetMathLibrary.MakeRotator` 0.0 (.pitch (`self.GetControlRotation`)) (.yaw (`self.GetControlRotation`)))) AxisValue)))

(event `RegenMax`
  ;[1 1 1] Die/Regen Event
  (set `self.Life` 100.0))

(event `InputAction|P2Interact`
  (params (Key :type "Key Structure"))
  ;[1 0.6223 0.5322] ActivateTurretMode
  (:`Pressed`
    (`/Engine/EditorBlueprintResources/StandardMacros.FlipFlop`
      (:`A`
        (if (`self.TurretOK?`)
          (set `self.Attach` true)
          (set `self.CalmDown` false)
          (`self.ReleaseTrigger`)
          (`self.ChangeColor`)))
      (:`B`
        (if (`self.Attach`)
          (set `self.Attach` false :!label _label_5)
          (`self.ReleaseTurret`)
          (`self.ChangeColor2`)
          (`KismetSystemLibrary.Delay` 1.0)
          (set `self.CalmDown` true))))))

(event `ChangeColor`
  ;[1 0.6223 0.5322] ActivateTurretMode
  (`PrimitiveComponent.SetCustomDepthStencilValue` (`self.Mesh`) 2)
  (`PrimitiveComponent.SetCustomDepthStencilValue` (`self.CapsuleComponent`) 2))

(event `DesactivateTurret`
  ;[1 0.6223 0.5322] ActivateTurretMode
  (goto _label_5))

(event `self.ReceiveTick`
  (params (DeltaSeconds :type "Float (single-precision)"))
  ;[0.4532 0.5476 1] EnergyGestion
  ;;[1 1 1] Energy Check
  (`KismetSystemLibrary.Delay` 0.8)
  (`|ExecutionSequence`
    (:`then_0`
      (if (and (`self.CalmDown`) (<= (`self.Energy`) 100.0))
        (`self.ReloadEnergy`)
        (elif (`self.Attach`)
          (`self.EnergyDownTurret`))))
    (:`then_1`
      (`KismetSystemLibrary.Delay` 1.0)
      (if (and (<= (`self.Shield`) 100.0) (>= (`self.Energy`) 1.0) (`self.CalmDown`))
        (`self.ReloadShield`)))
    (:`then_2`
      ;[0 0.6384 1] LifeGestion
      (if (and (< (`self.Life`) 100.0) (> (`self.Energy`) 0.0) (`self.CalmDown`))
        (`self.Regen`)))))

(event `ShieldDownTurret`
  ;[0.4532 0.5476 1] EnergyGestion
  ;;[1 1 1] Shield Down Turret
  (`KismetSystemLibrary.Delay` 0.2)
  (bind _output_get (set `self.Shield` (- (`self.Shield`) 4.0)))
  (`KismetSystemLibrary.PrintString` (`KismetStringLibrary.Conv_DoubleToString` _output_get))
  (if (<= (`self.Shield`) 0.0)
    (set `self.ShieldDown` true)
    (set `self.Attach` false)
    (`self.DesactivateTurret`)
    (set `self.Shield` 0.0)))

(event `InputAxis|GoDown`
  (params (AxisValue :type "Float (single-precision)"))
  ;[1 1 1] Go up / Go down
  (if (not (`self.Attach`))
    (`self.AddMovementInput` (`KismetMathLibrary.GetUpVector` (`KismetMathLibrary.MakeRotator` 0.0 (.pitch (`self.GetControlRotation`)) (.yaw (`self.GetControlRotation`)))) AxisValue)))

(event `ChangeColor2`
  ;[1 0.6223 0.5322] ActivateTurretMode
  (`PrimitiveComponent.SetCustomDepthStencilValue` (`self.Mesh`) 1)
  (`PrimitiveComponent.SetCustomDepthStencilValue` (`self.CapsuleComponent`) 1))

(event `PullTrigger`
  ;[0.4078 1 0.4995] ShootEvent
  (if (>= (`self.Energy`) 1.0)
    (set `self.DoShoot` true)
    (`/Engine/EditorBlueprintResources/StandardMacros.DoOnce` false :!label _label_6
      (:`Completed`
        (`self.Fire`)
        (`KismetSystemLibrary.K2_SetTimer` null "Fire" (/ 1.8 (`self.LaserPerSeconds`)) true)))))

(event `EnergyDownTurret`
  (bind _energy (`self.Energy`))
  ;[0.4532 0.5476 1] EnergyGestion
  ;;[1 1 1] Energy Down Turret
  (`KismetSystemLibrary.Delay` 0.2)
  (if (>= _energy 0.0)
    (bind _output_get (set `self.Energy` (- _energy 5.0)))
    (`KismetSystemLibrary.PrintString` (`KismetStringLibrary.Conv_DoubleToString` _output_get)))
  (if (and (<= (`self.Energy`) 0.0) (not (`self.ShieldDown`)))
    (set `self.Energy` 0.0)
    (`self.ShieldDownTurret`)
    (if (<= (`self.Shield`) 0.0)
      _)))

(event `InputAxis|Turn`
  (params (AxisValue :type "Float (single-precision)"))
  ;[1 1 1] Fly and turn
  (`self.AddControllerYawInput` AxisValue))

(event `PullTurret`
  ;[1 0.6223 0.5322] TurretMode
  (`/Engine/EditorBlueprintResources/StandardMacros.DoOnce` false :!label _label_7
    (:`Completed`
      (`self.FireTurret`)
      (`KismetSystemLibrary.K2_SetTimer` null "FireTurret" (/ 1.0 (`self.LaserPerSeconds`)) true))))

(event `ReloadEnergy`
  ;[0.4532 0.5476 1] EnergyGestion
  ;;[1 1 1] Reload Energy Event
  (set `self.Energy` (+ (`self.Energy`) 3.0))
  (if (>= (`self.Energy`) 100.0)
    (set `self.Energy` 100.0)))

(event `ReloadShield`
  (bind _shield (`self.Shield`))
  (bind _returnvalue (>= _shield 100.0))
  ;[0.4532 0.5476 1] EnergyGestion
  ;;[1 1 1] Reload Shield
  (if (not _returnvalue)
    (set `self.Shield` (+ _shield 6.0))
    (if _returnvalue
      (set `self.Shield` 100.0))))

(event `ReleaseTrigger`
  ;[0.4078 1 0.4995] ShootEvent
  (`KismetSystemLibrary.K2_ClearTimer` null "Fire")
  (`|ExecutionSequence`
    (:`then_0`
      (goto _label_6 :!via `Reset`))))

(event `ReleaseTurret`
  ;[1 0.6223 0.5322] TurretMode
  (`KismetSystemLibrary.K2_ClearTimer` null "FireTurret")
  (goto _label_7 :!via `Reset`))

(event `Fire`
  ;[0.4078 1 0.4995] ShootEvent
  (if (>= (`self.Energy`) 1.0)
    (`|SpawnActorFromClass` "/Game/PFE/Blueprint/BulletsOrWeapon/Bullets/Laser.Laser_C" (`SceneComponent.K2_GetComponentToWorld` (`self.ProjectileSpawnPoint`)) "Undefined" "OverrideRootScale" null null)
    (set `self.Energy` (- (`self.Energy`) 2.0))
    (set `self.DoShoot` true)))

(event `InputAxis|Lookup`
  (params (AxisValue :type "Float (single-precision)"))
  ;[1 1 1] Fly and turn
  (`self.AddControllerPitchInput` AxisValue))

(event `FireTurret`
  ;[1 0.6223 0.5322] TurretMode
  (if (or (>= (`self.Energy`) 1.0) (>= (`self.Shield`) 1.0))
    (`|SpawnActorFromClass` "/Game/PFE/Blueprint/BulletsOrWeapon/Bullets/LaserTurret.LaserTurret_C" (`SceneComponent.K2_GetComponentToWorld` (`self.ProjectileSpawnPoint`)) "Undefined" "OverrideRootScale" null null)
    (set `self.Energy` (- (`self.Energy`) 1.0))))

(fn `UserConstructionScript`)