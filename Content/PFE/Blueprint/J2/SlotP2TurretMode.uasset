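; SlotP2TurretMode is a turret slot whose activation is driven by overlaps from actors tagged Player1, despite the P2 in its name.
; Overlapping the Box toggles Sphere visibility and arms a SelectTurretActivate flag, which is never cleared here.
; Once armed, overlapping Sphere toggles Sphere1 visibility and enables its query and physics collision, the step labelled auto-turret activation.
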(event `self.Box.OnComponentBeginOverlap`
  (params (OverlappedComponent :type "PrimitiveComponent Object Reference") (OtherActor :type "Actor Object Reference") (OtherComp :type "PrimitiveComponent Object Reference") (OtherBodyIndex :type Integer) (bFromSweep :type Boolean) (SweepResult :type "HitResult Structure (by ref)"))
  ;[1 1 1] TurretRangeActivate
  (if (`self.ActorHasTag` OtherActor "Player1")
    (`SceneComponent.ToggleVisibility` (`self.Sphere`) false)
    (set `self.SelectTurretActivate` true)))

(event `self.Sphere.OnComponentBeginOverlap`
  (params (OverlappedComponent :type "PrimitiveComponent Object Reference") (OtherActor :type "Actor Object Reference") (OtherComp :type "PrimitiveComponent Object Reference") (OtherBodyIndex :type Integer) (bFromSweep :type Boolean) (SweepResult :type "HitResult Structure (by ref)"))
  ;[1 1 1] AutoTurret Active
  (if (and (`self.ActorHasTag` OtherActor "Player1") (`self.SelectTurretActivate`))
    (`SceneComponent.ToggleVisibility` (`self.Sphere1`) false)
    (`PrimitiveComponent.SetCollisionEnabled` (`self.Sphere1`) "QueryAndPhysics")))

(fn `UserConstructionScript`)