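; VR multiplayer game mode, judging by its name, that starts enemy spawning when play begins.
; BeginPlay takes the first EnemySpawner and first EnemySpawnerW2 in the level and sets looping timers by function name on their SpawnEnemy and Wave2 functions.
; Both timers start together and share an interval derived from EnemiesPerSeconds.
; An unconnected cast to GameInstance_PFE never runs.
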(event `self.ReceiveBeginPlay`
  (`|ExecutionSequence`
    (:`then_0`
      (bind _outactors (`GameplayStatics.GetAllActorsOfClass` "/Game/PFE/Blueprint/AI/AIGlobal/Spawner/EnemySpawner.EnemySpawner_C"))
      (bind _output_get (set `self.Spawner` (`|GetArrayItem` _outactors)))
      (`KismetSystemLibrary.K2_SetTimer` _output_get "SpawnEnemy" (/ 1.0 (`self.EnemiesPerSeconds`)) true))
    (:`then_1`
      (bind _outactors_2 (`GameplayStatics.GetAllActorsOfClass` "/Game/PFE/Blueprint/AI/AIGlobal/Spawner/EnemySpawnerW2.EnemySpawnerW2_C"))
      (bind _output_get_2 (set `self.SpawnerW2` (`|GetArrayItem` _outactors_2)))
      (`KismetSystemLibrary.K2_SetTimer` _output_get_2 "Wave2" (/ 1.0 (`self.EnemiesPerSeconds`)) true))))

(fn `UserConstructionScript`)