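; CristalSecret1 is a destructible secret crystal that reveals a hidden force field when it breaks.
; On BeginPlay it caches the first ForceFildHide1 actor found in the level.
; When the Destructible component fractures, it calls Reveal on that force field, then destroys itself after a short delay.
; An overlap check for the "Laser" tag is present but triggers nothing.
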(event `self.ReceiveBeginPlay`
  (bind _outactors (`GameplayStatics.GetAllActorsOfClass` "/Game/PFE/Blueprint/BulletsOrWeapon/Weapons/ForceFildHide1.ForceFildHide1_C"))
  (set `self.ForceField1` (`|GetArrayItem` _outactors)))

(event `self.ReceiveActorBeginOverlap`
  (params (OtherActor :type "Actor Object Reference"))
  (if (`self.ActorHasTag` OtherActor "Laser")
    _))

(event `self.Destructible.OnComponentFracture`
  (params (HitPoint :type "Vector Structure (by ref)") (HitDirection :type "Vector Structure (by ref)"))
  (`/Game/PFE/Blueprint/BulletsOrWeapon/Weapons/ForceFildHide1.Reveal` (`self.ForceField1`))
  (`KismetSystemLibrary.Delay` 10.0)
  (`self.K2_DestroyActor`))

(fn `UserConstructionScript`)