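; WeaponSelect is a hub interactable that reveals sword and claw buttons when touched by an actor tagged Hand.
; On BeginPlay it caches the PFE game instance, which is not otherwise used in these graphs.
; The first valid Sphere1 overlap toggles the widget's visibility, caches the world interaction pawn and shows both buttons.
; An Interact flag then blocks repeat triggers and is never reset here, and no selection logic is present.
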(event `self.ReceiveBeginPlay`
  (bind _asgame_instance_pfe (cast `/Game/PFE/Blueprint/GameInstance/GameInstance_PFE` (`GameplayStatics.GetGameInstance`)))
  (set `self.GI` _asgame_instance_pfe))

(event `self.Sphere1.OnComponentBeginOverlap`
  (params (OverlappedComponent :type "PrimitiveComponent Object Reference") (OtherActor :type "Actor Object Reference") (OtherComp :type "PrimitiveComponent Object Reference") (OtherBodyIndex :type Integer) (bFromSweep :type Boolean) (SweepResult :type "HitResult Structure (by ref)"))
  (if (and (`self.ActorHasTag` OtherActor "Hand") (not (`self.Interact`)))
    (`SceneComponent.ToggleVisibility` (`self.Widget`) false)
    (bind _asbp_world_interaction_pawn (cast `/Game/PFE/Blueprint/J1/BP_WorldInteractionPawn` (`GameplayStatics.GetPlayerPawn` 0)))
    (set `self.P1` _asbp_world_interaction_pawn)
    (`SceneComponent.SetVisibility` (`self.SwordButton`) true false)
    (`SceneComponent.SetVisibility` (`self.ClawButton`) true false)
    (set `self.Interact` true)))

(fn `UserConstructionScript`)