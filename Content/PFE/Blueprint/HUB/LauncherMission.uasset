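; VR hub mission launcher that starts Level1 when a player's hand touches its spheres in sequence.
; Overlapping Sphere1 with an actor tagged Hand reveals Sphere2 and Sphere3 and hides the widget.
; A hand overlap on Sphere3 swaps the material on Sphere and issues a servertravel console command to load Level1.
; Visibility alone stages the steps, with no state check before the travel.
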(event `self.Sphere1.OnComponentBeginOverlap`
  (params (OverlappedComponent :type "PrimitiveComponent Object Reference") (OtherActor :type "Actor Object Reference") (OtherComp :type "PrimitiveComponent Object Reference") (OtherBodyIndex :type Integer) (bFromSweep :type Boolean) (SweepResult :type "HitResult Structure (by ref)"))
  (if (`self.ActorHasTag` OtherActor "Hand")
    (`SceneComponent.SetVisibility` (`self.Sphere2`) true false)
    (`SceneComponent.SetVisibility` (`self.Sphere3`) true false)
    (`SceneComponent.SetVisibility` (`self.Widget`) false false)))

(event `self.Sphere3.OnComponentBeginOverlap`
  (params (OverlappedComponent :type "PrimitiveComponent Object Reference") (OtherActor :type "Actor Object Reference") (OtherComp :type "PrimitiveComponent Object Reference") (OtherBodyIndex :type Integer) (bFromSweep :type Boolean) (SweepResult :type "HitResult Structure (by ref)"))
  (if (`self.ActorHasTag` OtherActor "Hand")
    (`PrimitiveComponent.SetMaterial` (`self.Sphere`) 0 "/Game/PFE/Blueprint/BulletsOrWeapon/Bullets/Materials/LaserMatTurret.LaserMatTurret")
    (`KismetSystemLibrary.ExecuteConsoleCommand` "servertravel /Game/PFE/Levels/Level1" null)))

(fn `UserConstructionScript`)