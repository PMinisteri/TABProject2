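; UpgradeShop is a hub Blueprint for an upgrade shop, currently containing only proximity-triggered display logic.
; When an actor tagged Player1 enters Sphere1, it toggles visibility on the cube, widget and two static meshes.
; It then casts its existing P1 reference to BP_WorldInteractionPawn and stores it back.
; The other sphere and cube overlap handlers do nothing, and no upgrade or purchase logic is present.
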(event `self.Sphere.OnComponentBeginOverlap`
  (params (OverlappedComponent :type "PrimitiveComponent Object Reference") (OtherActor :type "Actor Object Reference") (OtherComp :type "PrimitiveComponent Object Reference") (OtherBodyIndex :type Integer) (bFromSweep :type Boolean) (SweepResult :type "HitResult Structure (by ref)")))

(event `self.Sphere1.OnComponentBeginOverlap`
  (params (OverlappedComponent :type "PrimitiveComponent Object Reference") (OtherActor :type "Actor Object Reference") (OtherComp :type "PrimitiveComponent Object Reference") (OtherBodyIndex :type Integer) (bFromSweep :type Boolean) (SweepResult :type "HitResult Structure (by ref)"))
  (if (`self.ActorHasTag` OtherActor "Player1")
    (`SceneComponent.ToggleVisibility` (`self.Cube`) false)
    (`SceneComponent.ToggleVisibility` (`self.Widget`) false)
    (`SceneComponent.ToggleVisibility` (`self.StaticMesh1`) false)
    (`SceneComponent.ToggleVisibility` (`self.StaticMesh`) false)
    (bind _asbp_world_interaction_pawn (cast `/Game/PFE/Blueprint/J1/BP_WorldInteractionPawn` (`self.P1`)))
    (set `self.P1` _asbp_world_interaction_pawn)))

(event `self.Cube.OnComponentBeginOverlap`
  (params (OverlappedComponent :type "PrimitiveComponent Object Reference") (OtherActor :type "Actor Object Reference") (OtherComp :type "PrimitiveComponent Object Reference") (OtherBodyIndex :type Integer) (bFromSweep :type Boolean) (SweepResult :type "HitResult Structure (by ref)"))
  (if (`self.ActorHasTag` OtherActor "Player1")
    _))

(fn `UserConstructionScript`)