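; BP_Soldier is an AI-controlled enemy soldier that shoots lasers at the player.
; A looping one-second timer calls Fire, which spawns a LaserIA at the Arrow component when the player is within range and the soldier is alive.
; An empty magazine triggers a delayed Reload, mirrored to the isReloading Blackboard key for the AI.
; The Die event is an empty stub.
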(event `self.ReceiveBeginPlay`
  (`KismetSystemLibrary.K2_SetTimer` null "Fire" 1.0 true))

(event `Reload`
  (if (not (or (`self.IsReloading`) (`self.IsDead`)))
    (`BlackboardComponent.SetValueAsBool` (`AIBlueprintHelperLibrary.GetBlackboard` (`self.GetController`)) "isReloading" true)
    (set `self.IsReloading` true)
    (`KismetSystemLibrary.Delay` 2.5)
    (set `self.AmmoInMag` (`self.MaxAmmoInMag`))
    (set `self.IsReloading` false)
    (`BlackboardComponent.SetValueAsBool` (`AIBlueprintHelperLibrary.GetBlackboard` (`self.GetController`)) "isReloading" false)))

(event `Fire`
  (if (`self.IsDead`)
    _
    (elif (== (`self.AmmoInMag`) 0)
      (`self.Reload`)
      (elif (< (`KismetMathLibrary.VSize` (- (`self.K2_GetActorLocation` (`GameplayStatics.GetPlayerPawn` 0)) (`self.K2_GetActorLocation`))) 1000.0)
        (`|SpawnActorFromClass` "/Game/PFE/Blueprint/BulletsOrWeapon/Bullets/LaserIA.LaserIA_C" (`SceneComponent.K2_GetComponentToWorld` (`self.Arrow`)) "Undefined" "OverrideRootScale" null null)
        (set `self.AmmoInMag` (- (`self.AmmoInMag`) 1))))))

(event `Die`)

(fn `UserConstructionScript`
  (`parent.UserConstructionScript`))