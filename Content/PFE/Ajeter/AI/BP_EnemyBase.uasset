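; Base enemy Blueprint that loses Life when hit by tagged attacks and enables physics on its skeletal mesh once Life runs out.
; Capsule overlaps scale damage by tag, from lasers and turret lasers to light claw or hand hits, while Sphere laser overlaps deal the heaviest damage.
; The LaserVR check reads the enemy's own tags rather than the overlapping actor's.
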(event `self.Capsule.OnComponentBeginOverlap`
  (params (OverlappedComponent :type "PrimitiveComponent Object Reference") (OtherActor :type "Actor Object Reference") (OtherComp :type "PrimitiveComponent Object Reference") (OtherBodyIndex :type Integer) (bFromSweep :type Boolean) (SweepResult :type "HitResult Structure (by ref)"))
  (if (or (`self.ActorHasTag` OtherActor "Laser") (`ActorComponent.ComponentHasTag` OtherComp "Laser"))
    (set `self.Life` (- (`self.Life`) 10.0))
    (if (<= (`self.Life`) 0.0) :!label _label
      (`PrimitiveComponent.SetSimulatePhysics` (`self.SkeletalMesh`) true))
    (elif (or (`self.ActorHasTag` "LaserVR") (`self.ActorHasTag` OtherActor "LaserTurret"))
      (set `self.Life` (- (`self.Life`) 30.0))
      (goto _label)
      (elif (`self.ActorHasTag` OtherActor "Scan")
        _
        (elif (or (`self.ActorHasTag` OtherActor "Claw") (`ActorComponent.ComponentHasTag` OtherComp "Hand"))
          (set `self.Life` (- (`self.Life`) 1.0))
          (goto _label))))))

(event `self.Sphere.OnComponentBeginOverlap`
  (params (OverlappedComponent :type "PrimitiveComponent Object Reference") (OtherActor :type "Actor Object Reference") (OtherComp :type "PrimitiveComponent Object Reference") (OtherBodyIndex :type Integer) (bFromSweep :type Boolean) (SweepResult :type "HitResult Structure (by ref)"))
  (if (`self.ActorHasTag` OtherActor "Laser")
    (set `self.Life` (- (`self.Life`) 50.0))
    (goto _label)))

(fn `UserConstructionScript`)